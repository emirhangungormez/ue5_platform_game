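; BP_Platfrom is a moving platform that collapses some time after something overlaps its trigger box.
; The construction script turns the spline's second point into a relative InterpToMovement target from the origin and applies the exposed Duration.
; On overlap, with no actor filter, it plays a world camera shake at the player pawn's location, then enables physics simulation on the platform mesh after a fixed delay.
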(event OnComponentBeginOverlap(trigger_box)
  (params (OverlappedComponent :type Primitive%20Component%20Object%20Reference) (OtherActor :type Actor%20Object%20Reference) (OtherComp :type Primitive%20Component%20Object%20Reference) (OtherBodyIndex :type Integer) (bFromSweep :type Boolean) (SweepResult :type Hit%20Result%20Structure%20%28by%20ref%29))
  (Camera|PlayWorldCameraShake "/Game/MyPlatformGame/BP_Camera.BP_Camera_C" (Transformation|GetActorLocation (Game|Player|GetPlayerPawn 0)) 2e+02 1e+03)
  (Utilities|FlowControl|Delay 7.0)
  (Physics|SetSimulatePhysics (Variables|Default|GetSM_Platfrom) true))

(event EventBeginPlay)

(event Collision|EventActorBeginOverlap
  (params (OtherActor :type Actor%20Object%20Reference)))

(event EventTick
  (params (DeltaSeconds :type Float%20%28single-precision%29)))

(fn ConstructionScript
  (Variables|/Script/Engine.InterpToMovementComponent|SetControlPoints (Variables|Default|GetInterpToMovement) (Utilities|Array|MakeArray (Utilities|Struct|MakeInterpControlPoint "0.000000,0.000000,0.000000" true) (Utilities|Struct|MakeInterpControlPoint (Spline|GetLocationatSplinePoint (Variables|Default|GetSpline) 1 "Local") true)))
  (Variables|/Script/Engine.InterpToMovementComponent|SetDuration (Variables|Default|GetInterpToMovement) (Variables|Default|GetDuration)))